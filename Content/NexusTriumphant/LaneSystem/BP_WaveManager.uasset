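; Lane wave manager that spawns BP_Minion waves from both ends of a spline and gives movement targets along it.
; BeginPlay runs a single wave of five spawn pairs, one second apart, with the far-end minion flipped and set to TeamRight.
; GetMoveToLocation projects a location onto the spline and steps a given distance forward or backward by team, clamped to the spline's length.
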(event Custom|OnWave
  (bind _spline (Variables|Default|GetSpline))
  (bind _spline_2 (Variables|Default|GetSpline))
  (bind _returnvalue (Spline|GetTransformatSplinePoint _spline_2 0 "World" false))
  (bind _returnvalue_2 (Spline|GetNumberOfSplinePoints _spline))
  (bind _returnvalue_3 (- _returnvalue_2 1))
  (bind _returnvalue_4 (Spline|GetTransformatSplinePoint _spline _returnvalue_3 "World" false))
  (Variables|Default|SetMinionIter 0)
  (if (< (Variables|Default|GetMinionIter) 5) :!label _label
    (Utilities|FlowControl|Delay 1.0)
    (Utilities|FlowControl|Sequence
      (:then_0
        (Game|SpawnActorfromClass "/Game/NexusTriumphant/Entities/Minions/BP_Minion.BP_Minion_C" (Math|Transform|MakeTransform (.location _returnvalue) (.rotation _returnvalue) "1.000000,1.000000,1.000000") "AdjustIfPossibleButAlwaysSpawn" "MultiplyWithRoot" 0 self "NewEnumerator0" 0))
      (:then_1
        (Game|SpawnActorfromClass "/Game/NexusTriumphant/Entities/Minions/BP_Minion.BP_Minion_C" (Math|Transform|MakeTransform (.location _returnvalue_4) (Math|Rotator|CombineRotators (.rotation _returnvalue_4) "0.000000,180.000000,0.000000") "1.000000,1.000000,1.000000") "AdjustIfPossibleButAlwaysSpawn" "MultiplyWithRoot" 0 self "NewEnumerator1" 0))
      (:then_2
        (Math|Integer|IncrementInt (Variables|Default|GetMinionIter)
          (:%20%20
            (goto _label)))))))

(event EventBeginPlay
  (Variables|Default|SetMinionHalfHeight 55.0)
  (CallFunction|OnWave))

(fn ConstructionScript)

(fn GetMovetoLocation
  (params (InLocation :type Vector%20%28by%20ref%29) (Distance :type Float%20%28double-precision%29) (Team :type ETeam%20Enum :default "NewEnumerator2"))
  (bind _map (Utilities|Map|MakeMap "NewEnumerator0" 1 "NewEnumerator1" -1))
  (bind _spline (Variables|Default|GetSpline))
  (bind (_value _returnvalue) (Utilities|Map|Find _map Team))
  (if _returnvalue
    _
    (else
      (Development|PrintString "Warning: Invalid team passed to GetMovetoLocation, BP_WaveManager ")))
  (return (Spline|GetLocationatDistanceAlongSpline _spline (Math|Float|Clamp(Float) (+ (Class|SplineComponent|GetDistanceAlongSplineatLocation (Variables|Default|GetSpline) InLocation "World") (* Distance _value)) 0.0 (Spline|GetSplineLength _spline)) "World")))