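; Minion character that stores its wave manager's spline as its path and is set up to bounce off overlapping characters.
; Each tick, a capsule overlap query finds characters, stops the minion's movement while keeping its pathing, and applies velocity-change impulses from GetBounceVector.
; Other minions also receive a horizontal impulse.
; GetBounceVector's direction-and-radius calculation is left unconnected, and the debug print chains never run.
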(event EventTick
  (params (DeltaSeconds :type Float%20%28single-precision%29))
  (bind _charactermovement (Variables|Character|GetCharacterMovement))
  (bind _bounce_overlap_capsule (Variables|Default|GetBounce%20Overlap%20Capsule))
  (bind (_outactors _returnvalue) (Collision|ComponentOverlapActors _bounce_overlap_capsule (Transformation|GetWorldTransform _bounce_overlap_capsule) (Utilities|Array|MakeArray "ObjectTypeQuery8" "ObjectTypeQuery9") 0 (Utilities|Array|MakeArray self)))
  (for _array_element _outactors
    (bind _ascharacter (Utilities|Casting|CastToCharacter _array_element))
    (if (.bSuccess (Utilities|Casting|CastToBP_Minion _ascharacter))
      (Physics|AddImpulse (Variables|/Script/Engine.Character|GetCharacterMovement _ascharacter) (* (Utilities|GetBounceVector _ascharacter self 1.0) "1.000000,1.000000,0.000000") true))
    (Class|NavMovementComponent|StopMovementKeepPathing _charactermovement)
    (Physics|AddImpulse _charactermovement (Utilities|GetBounceVector self _ascharacter 1e+01) true)))

(event EventBeginPlay
  (bind _wave_manager (Variables|Default|GetWave%20Manager))
  (Utilities|IsValid _wave_manager
    (:Is%20Valid
      (Variables|Default|SetPath (Variables|/Game/NexusTriumphant/LaneSystem/BP_WaveManager.BP_WaveManager_C|GetSpline _wave_manager)))))

(fn ConstructionScript)