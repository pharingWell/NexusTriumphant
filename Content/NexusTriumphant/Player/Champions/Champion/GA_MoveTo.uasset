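; Gameplay ability that moves a champion to a target point when activated by a gameplay event from an NPlayerController instigator.
; It commits, then takes the blocking hit from the event's target data, falling back to a Visibility trace under the cursor.
; SimpleMoveToLocation starts the move and the ability ends immediately without waiting for arrival, leaving debug prints on success and failure.
; Activation without event data just ends the ability.
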(event Ability|EventActivateAbility
  (Ability|EndAbility))

(event Ability|EventOnEndAbility
  (params (bWasCancelled :type Boolean)))

(event Ability|EventActivateAbilityFromEvent
  (params (EventData :type Gameplay%20Event%20Data%20Structure%20%28by%20ref%29))
  (bind (_eventtag _instigator _target _optionalobject _optionalobject2 _contexthandle _instigatortags _targettags _eventmagnitude _targetdata) (Utilities|Struct|BreakGameplayEventData EventData))
  (bind _returnvalue (Ability|TargetData|GetHitResultfromTargetData _targetdata))
  (|CallParentFunction EventData)
  (Ability|CommitAbility)
  (bind _asnplayer_controller (Utilities|Casting|CastToNPlayerController _instigator)
    (:then
      (if (Ability|TargetData|TargetDataHasHitResult _targetdata)
        (if (.bBlockingHit (Collision|BreakHitResult _returnvalue))
          (Variables|Default|SetHitResult _returnvalue)
          (Development|PrintString "Hello, World" :!label _label)
          (AI|Navigation|SimpleMovetoLocation _asnplayer_controller (.Location (Collision|BreakHitResult (Variables|Default|GetHitResult))))
          (Ability|EndAbility)
          (else
            (bind (_hitresult _returnvalue_2) (Class|NPlayerController|GetHitResultUnderCursor _asnplayer_controller "ECC_Visibility" false :!label _label_2))
            (if _returnvalue_2
              (Variables|Default|SetHitResult _hitresult)
              (goto _label)
              (else
                (Development|PrintString "Else" :!label _label_3)
                (Ability|EndAbility)))))
        (else
          (goto _label_2))))
    (:CastFailed
      (goto _label_3))))